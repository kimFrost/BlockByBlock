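; Player controller for a side-scroller with Mine and Build tools, mapping the mouse onto the X-normal gameplay plane.
; Each tick it traces a short ray from the character toward the cursor to target and highlight blocks, and draws a grid-snapped debug box.
; Left click either picks up the targeted block or releases the held one into a free slot, or in Build sets two points for a belt.
; Q selects Build.
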(event `self.ReceiveTick`
  (params (DeltaSeconds :type "Float (single-precision)"))
  (bind (_worldlocation _worlddirection) (`self.DeprojectMousePositionToWorld`))
  (bind (_worldlocation_2 _worlddirection_2) (`self.DeprojectMousePositionToWorld`))
  (bind _blockhighlighter (`self.BlockHighlighter`))
  (bind _blockhighlighter_2 (`self.BlockHighlighter`))
  (`|ExecutionSequence`
    (:`then_0`
      (bind _asside_scroller_character (cast `/Game/SideScrollerCPP/Blueprints/SideScrollerCharacter` (`self.K2_GetPawn`)))
      (bind _returnvalue (`self.K2_GetActorLocation` _asside_scroller_character))
      (bind (_outhit _returnvalue_2) (`KismetSystemLibrary.LineTraceSingle` :`Start` _returnvalue :`End` (+ _returnvalue (* (`KismetMathLibrary.GetDirectionUnitVector` _returnvalue (`.Intersection` (`KismetMathLibrary.LinePlaneIntersection_OriginNormal` _worldlocation (+ _worldlocation (* _worlddirection 100000.0)) (0.0 0.0 0.0) (1.0 0.0 0.0)))) 200.0)) :`TraceChannel` "TraceTypeQuery3" :`bTraceComplex` true :`DrawDebugType` "ForOneFrame" :`DrawTime` 0.0))
      (if _returnvalue_2
        (bind _asbp_block (cast `/Game/Blueprint/Actors/BP_Block` (`.HitActor` (`GameplayStatics.BreakHitResult` _outhit)))
          (:`then`
            (set `self.TargetedBlock` _asbp_block)
            (`/Engine/EditorBlueprintResources/StandardMacros.IsValid` _blockhighlighter_2
              (:`Is Valid`
                (`self.K2_DestroyActor` _blockhighlighter_2))
              (:`Is Not Valid`
                _))
            (bind _returnvalue_3 (`|SpawnActorFromClass` "/Game/Blueprint/Actors/BP_HighlightBlock.BP_HighlightBlock_C" (`self.GetTransform` _asbp_block) "Undefined" "OverrideRootScale"))
            (set `self.BlockHighlighter` _returnvalue_3))
          (:`CastFailed`
            (set `self.TargetedBlock` null :!label _label)
            (`/Engine/EditorBlueprintResources/StandardMacros.IsValid` _blockhighlighter
              (:`Is Valid`
                (`self.K2_DestroyActor` _blockhighlighter)))))
        (else
          (goto _label))))
    (:`then_1`
      (`KismetSystemLibrary.DrawDebugBox` (+ (`/Game/Blueprint/Util/BPFL_Grid.RoundLocationToGrid` (`.Intersection` (`KismetMathLibrary.LinePlaneIntersection_OriginNormal` _worldlocation_2 (+ _worldlocation_2 (* _worlddirection_2 100000.0)) (35.0 0.0 0.0) (1.0 0.0 0.0)))) (0.0 0.0 35.0)) (35.0 35.0 35.0) (struct :`G` 0.622144 :`B` 1.0 :`A` 1.0) (struct) 0.0 5.0))))

(event `Key|LeftMouseButton`
  (params (Key :type "Key Structure" :default "AnyKey"))
  (bind (_worldlocation _worlddirection) (`self.DeprojectMousePositionToWorld`))
  (bind _buildfrom (`self.BuildFrom`))
  (bind _gridlocation (`/Game/Blueprint/Util/BPFL_Grid.RoundLocationToGrid` (`.Intersection` (`KismetMathLibrary.LinePlaneIntersection_OriginNormal` _worldlocation (+ _worldlocation (* _worlddirection 100000.0)) (0.0 0.0 0.0) (1.0 0.0 0.0)))))
  (:`Pressed`
    (switch `/Game/Util/Enums/EToolType` (`self.CurrentTool`)
      (:`NewEnumerator0`
        (bind _asside_scroller_character (cast `/Game/SideScrollerCPP/Blueprints/SideScrollerCharacter` (`self.K2_GetPawn`)))
        (`/Engine/EditorBlueprintResources/StandardMacros.IsValid` (`self.TargetedBlock`)
          (:`Is Valid`
            (`/Game/SideScrollerCPP/Blueprints/SideScrollerCharacter.PickupBlock` _asside_scroller_character (`self.TargetedBlock`)))
          (:`Is Not Valid`
            (bind _asbp_block_slot (cast `/Game/Blueprint/Actors/BP_BlockSlot` (`.HitActor` (`GameplayStatics.BreakHitResult` (`self.GetHitResultUnderCursorByChannel` "TraceTypeQuery1")))))
            (bind _isfree (`/Game/Blueprint/Actors/BP_BlockSlot.IsFree` _asbp_block_slot))
            (if _isfree
              (bind _asbp_block_slot_2 (cast `/Game/Blueprint/Actors/BP_BlockSlot` (`ChildActorComponent.ChildActor` (`/Game/SideScrollerCPP/Blueprints/SideScrollerCharacter.BlockSlot` _asside_scroller_character))))
              (bind (_breleased _releasedblock) (`/Game/Blueprint/Actors/BP_BlockSlot.ReleaseBlock` _asbp_block_slot_2 false))
              (if _breleased
                (`/Game/Blueprint/Actors/BP_BlockSlot.AddBlock` _asbp_block_slot _releasedblock))))))
      (:`NewEnumerator1`
        (if (`self.BuildFirstPlaced`)
          (set `self.BuildTo` _gridlocation)
          (set `self.BuildFirstPlaced` false)
          (`|SpawnActorFromClass` "/Game/Blueprint/Actors/BP_Belt.BP_Belt_C" (`KismetMathLibrary.MakeTransform` _buildfrom) "Undefined" "OverrideRootScale" null _buildfrom (`self.BuildTo`))
          (else
            (set `self.BuildFrom` _gridlocation)
            (set `self.BuildFirstPlaced` true)))))))

(event `Key|Q`
  (params (Key :type "Key Structure" :default "AnyKey"))
  (:`Pressed`
    (`self.SwitchTool` "NewEnumerator1")))

(fn `SwitchTool`
  (params (ToolType :type "/Game/Util/Enums/EToolType Enum"))
  (switch `/Game/Util/Enums/EToolType` ToolType
    (:`NewEnumerator0`
      _)
    (:`NewEnumerator1`
      _))
  (set `self.CurrentTool` ToolType))

(fn `UserConstructionScript`)