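; Test rope actor that physically tethers its static mesh to a TetherTo actor, with a Cable component's end attached to that actor.
; On BeginPlay, UpdateRope spawns a downward line of simulated sphere joints and chains them with physics constraints from the mesh to the target's root, which must be a StaticMeshComponent.
; The construction script holds a disconnected copy of this logic, and UpdateAttachment is an empty stub.
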(event `self.ReceiveBeginPlay`
  (`self.UpdateRope`))

(fn `UpdateAttachment`)

(fn `UpdateRope`
  (bind _joints (`self.Joints`))
  (bind _joints_2 (`self.Joints`))
  (bind _tetherto (`self.TetherTo`))
  (bind _item (`KismetArrayLibrary.Array_Get` _joints_2 (`KismetArrayLibrary.Array_LastIndex` _joints_2)))
  (`/Engine/EditorBlueprintResources/StandardMacros.IsValid` _tetherto
    (:`Is Valid`
      (`CableComponent.SetAttachEndTo` (`self.Cable`) _tetherto "None" "None")
      (`KismetArrayLibrary.Array_Clear` (`self.Joints`))
      (`|ExecutionSequence`
        (:`then_0`
          (for _index (range 1 (+ (`self.NumOfJoints`) 1))
            (bind _returnvalue (`AddComponent|NODE_AddSphereComponent-2` :`bManualAttachment` true :`RelativeTransform` (`KismetMathLibrary.MakeTransform` (`KismetMathLibrary.MakeVector` 0.0 0.0 (+ (* _index -50.0) -50.0)))))
            (`SceneComponent.K2_AttachToComponent` _returnvalue (`self.StaticMesh`) "None" "KeepRelative" "KeepRelative" "KeepRelative" true)
            (`PrimitiveComponent.SetCollisionObjectType` _returnvalue "ECC_PhysicsBody")
            (`PrimitiveComponent.SetCollisionResponseToAllChannels` _returnvalue "ECR_Block")
            (`PrimitiveComponent.SetCollisionEnabled` _returnvalue "QueryAndPhysics")
            (`PrimitiveComponent.SetCollisionProfileName` _returnvalue "PhysiscActor")
            (`PrimitiveComponent.SetSimulatePhysics` _returnvalue true)
            (`SphereComponent.SetSphereRadius` _returnvalue (`self.RobeRadius`) true)
            (`KismetArrayLibrary.Array_Add` (`self.Joints`) _returnvalue)))
        (:`then_1`
          (`|ExecutionSequence`
            (:`then_0`
              (bind _returnvalue_2 (`AddComponent|NODE_AddPhysicsConstraintComponent-5` :`bManualAttachment` true :`RelativeTransform` (`KismetMathLibrary.MakeTransform` (0.0 0.0 0.0))))
              (`SceneComponent.K2_AttachToComponent` _returnvalue_2 (`self.StaticMesh`) "None" "KeepRelative" "KeepRelative" "KeepRelative" true)
              (`PhysicsConstraintComponent.SetConstrainedComponents` _returnvalue_2 (`self.StaticMesh`) "None" (`KismetArrayLibrary.Array_Get` (`self.Joints`)) "None"))
            (:`then_1`
              (for _index_2 (range (`KismetArrayLibrary.Array_LastIndex` (`self.Joints`)))
                (bind _returnvalue_3 (`AddComponent|NODE_AddPhysicsConstraintComponent-4` :`bManualAttachment` true :`RelativeTransform` (`KismetMathLibrary.MakeTransform` (0.0 0.0 0.0))))
                (bind _item_2 (`KismetArrayLibrary.Array_Get` _joints _index_2))
                (`SceneComponent.K2_AttachToComponent` _returnvalue_3 _item_2 "None" "KeepRelative" "KeepRelative" "KeepRelative" true)
                (`PhysicsConstraintComponent.SetConstrainedComponents` _returnvalue_3 _item_2 "None" (`KismetArrayLibrary.Array_Get` _joints (+ _index_2 1)) "None")))
            (:`then_2`
              (bind _asstatic_mesh_component (cast `StaticMeshComponent` (`self.K2_GetRootComponent` (`self.TetherTo`))))
              (bind _returnvalue_4 (`AddComponent|NODE_AddPhysicsConstraintComponent-6` :`bManualAttachment` true :`RelativeTransform` (`KismetMathLibrary.MakeTransform` (0.0 0.0 0.0))))
              (`SceneComponent.K2_AttachToComponent` _returnvalue_4 _item "None" "KeepRelative" "KeepRelative" "KeepRelative" true)
              (`PhysicsConstraintComponent.SetConstrainedComponents` _returnvalue_4 _item "None" _asstatic_mesh_component "None"))))))))

(fn `UserConstructionScript`)