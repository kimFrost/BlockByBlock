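; BP_BlockOrganizer is a utility actor that snaps every BP_Block in the level to a 100-unit grid.
; Its construction script finds all blocks and rounds each location axis to the nearest multiple of 100, moving them without sweep.
; The script also resets an Update boolean to false, which suggests a checkbox used as a re-run button.
; The event graph has no active logic.
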(fn `UserConstructionScript`
  (set `self.Update` false)
  (bind _outactors (`GameplayStatics.GetAllActorsOfClass` "/Game/Blueprint/Actors/BP_Block.BP_Block_C"))
  (for _array_element _outactors
    (`self.K2_SetActorLocation` _array_element (* (`KismetMathLibrary.MakeVector` (`KismetMathLibrary.Conv_IntToDouble` (`KismetMathLibrary.Round` (.x (/ (`self.K2_GetActorLocation` _array_element) 100.0)))) (`KismetMathLibrary.Conv_IntToDouble` (`KismetMathLibrary.Round` (.y (/ (`self.K2_GetActorLocation` _array_element) 100.0)))) (`KismetMathLibrary.Conv_IntToDouble` (`KismetMathLibrary.Round` (.z (/ (`self.K2_GetActorLocation` _array_element) 100.0))))) 100.0) false false)))