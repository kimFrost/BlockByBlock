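; BP_Tether is an actor that visually links a TetherFrom actor to a TetherTo actor with a cable.
; On BeginPlay, if both references are valid, Tether stores them, attaches the cable end to TetherTo, then casts them to SideScrollerCharacter and BP_Block.
; The physics tether is unfinished: constraint and grab nodes are disconnected, and the constraint update and clear functions have no effect.
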(event `self.ReceiveBeginPlay`
  (`/Engine/EditorBlueprintResources/StandardMacros.IsValid` (`self.TetherFrom`)
    (:`Is Valid`
      (`/Engine/EditorBlueprintResources/StandardMacros.IsValid` (`self.TetherTo`)
        (:`Is Valid`
          (`self.Tether` (`self.TetherFrom`) (`self.TetherTo`)))
        (:`Is Not Valid`
          (`KismetSystemLibrary.PrintString` "34234234"))))))

(event `self.ReceiveTick`
  (params (DeltaSeconds :type "Float (single-precision)")))

(fn `_ClearConstraints`)

(fn `Tether`
  (params (TetherFrom :type "Actor Object Reference") (TetherTo :type "Actor Object Reference"))
  (set `self.TetherFrom` TetherFrom)
  (set `self.TetherTo` TetherTo)
  (`CableComponent.SetAttachEndTo` (`self.Cable`) (`self.TetherTo`) "None" "None")
  (bind _asside_scroller_character (cast `/Game/SideScrollerCPP/Blueprints/SideScrollerCharacter` (`self.TetherFrom`)))
  (bind _asbp_block (cast `/Game/Blueprint/Actors/BP_Block` (`self.TetherTo`))))

(fn `TetherOld`
  (params (Comp1 :type "PrimitiveComponent Object Reference") (Comp2 :type "PrimitiveComponent Object Reference")))

(fn `UpdateConstraints`
  (`self._ClearConstraints`)
  (if (> (`self.Length`) 0.0)
    _))

(fn `UserConstructionScript`)