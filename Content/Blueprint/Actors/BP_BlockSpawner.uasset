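; BP_BlockSpawner is an actor that builds a wall-like grid of BP_Block actors when play begins, unless SpawnInConstruction is set.
; BeginPlay runs nested loops over Rows and Columns, spawning widened blocks at fixed spacing in the XZ plane with physics simulation and trace pickup disabled.
; Positions are absolute world coordinates, independent of the spawner's transform.
; The construction script is empty, so enabling that flag spawns nothing here.
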(event `self.ReceiveBeginPlay`
  (if (not (`self.SpawnInConstruction`))
    (`|ExecutionSequence`
      (:`then_1`
        (for _index (range (+ (`self.Rows`) 1))
          (for _index_2 (range (+ (`self.Columns`) 1))
            (`|SpawnActorFromClass` "/Game/Blueprint/Actors/BP_Block.BP_Block_C" (`KismetMathLibrary.MakeTransform` (`KismetMathLibrary.MakeVector` (+ (* _index_2 70.0) 500.0) 0.0 (* _index 70.0)) (struct) (1.0 1.5 1.0)) "Undefined" "OverrideRootScale")))))))

(fn `UserConstructionScript`)