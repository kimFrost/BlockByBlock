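; Dev test rope actor that tethers two actors, each a SideScrollerCharacter or BP_Block, with a simulated physics chain.
; UpdateReferences resolves each end's mesh during construction and at BeginPlay, then UpdateRope spawns simulated sphere joints below the start, linked by runtime-created physics constraints.
; A Cable component connects the endpoints directly, independent of the joints.
; The final constraint requires a StaticMeshComponent, so a character's skeletal mesh at the far end stays unconstrained.
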(event `self.ReceiveBeginPlay`
  (`self.UpdateReferences`)
  (`self.UpdateRope`))

(fn `UpdateAttachment`)

(fn `UpdateReferences`
  (bind _tetherto (`self.TetherTo`))
  (bind _tetherfrom (`self.TetherFrom`))
  (`|ExecutionSequence`
    (:`then_0`
      (bind _asside_scroller_character (cast `/Game/SideScrollerCPP/Blueprints/SideScrollerCharacter` _tetherfrom)
        (:`then`
          (set `self.TetherFromComp` (`Character.Mesh` _asside_scroller_character)))
        (:`CastFailed`
          (bind _asbp_block (cast `/Game/Blueprint/Actors/BP_Block` _tetherfrom))
          (set `self.TetherFromComp` (`/Game/Blueprint/Actors/BP_Block.StaticMesh` _asbp_block)))))
    (:`then_1`
      (bind _asside_scroller_character_2 (cast `/Game/SideScrollerCPP/Blueprints/SideScrollerCharacter` _tetherto)
        (:`then`
          (set `self.TetherToComp` (`Character.Mesh` _asside_scroller_character_2)))
        (:`CastFailed`
          (bind _asbp_block_2 (cast `/Game/Blueprint/Actors/BP_Block` _tetherto))
          (set `self.TetherToComp` (`/Game/Blueprint/Actors/BP_Block.StaticMesh` _asbp_block_2)))))))

(fn `UpdateRope`
  (bind _joints (`self.Joints`))
  (bind _joints_2 (`self.Joints`))
  (bind _item (`KismetArrayLibrary.Array_Get` _joints_2 (`KismetArrayLibrary.Array_LastIndex` _joints_2)))
  (`/Engine/EditorBlueprintResources/StandardMacros.IsValid` (`self.TetherFromComp`)
    (:`Is Valid`
      (`/Engine/EditorBlueprintResources/StandardMacros.IsValid` (`self.TetherToComp`)
        (:`Is Valid`
          (`SceneComponent.K2_AttachToComponent` (`self.Cable`) (`self.TetherFromComp`) "None" "KeepWorld" "KeepRelative" "KeepRelative" true)
          (`CableComponent.SetAttachEndTo` (`self.Cable`) (`self.TetherTo`) "None" "None")
          (`KismetArrayLibrary.Array_Clear` (`self.Joints`))
          (`|ExecutionSequence`
            (:`then_0`
              (for _index (range 1 (+ (`self.NumOfJoints`) 1))
                (bind _returnvalue (`AddComponent|NODE_AddSphereComponent-2` :`bManualAttachment` true :`RelativeTransform` (`KismetMathLibrary.MakeTransform` (`KismetMathLibrary.MakeVector` 0.0 0.0 (+ (* _index -50.0) -50.0)))))
                (`SceneComponent.K2_AttachToComponent` _returnvalue (`self.TetherFromComp`) "None" "KeepRelative" "KeepRelative" "KeepRelative" true)
                (`PrimitiveComponent.SetCollisionObjectType` _returnvalue "ECC_PhysicsBody")
                (`PrimitiveComponent.SetCollisionResponseToAllChannels` _returnvalue "ECR_Block")
                (`PrimitiveComponent.SetCollisionEnabled` _returnvalue "QueryAndPhysics")
                (`PrimitiveComponent.SetCollisionProfileName` _returnvalue "PhysiscActor")
                (`PrimitiveComponent.SetSimulatePhysics` _returnvalue true)
                (`SphereComponent.SetSphereRadius` _returnvalue (`self.RobeRadius`) true)
                (`KismetArrayLibrary.Array_Add` (`self.Joints`) _returnvalue)
                (`SceneComponent.SetHiddenInGame` _returnvalue false false)))
            (:`then_1`
              (`|ExecutionSequence`
                (:`then_0`
                  (bind _returnvalue_2 (`AddComponent|NODE_AddPhysicsConstraintComponent-5` :`bManualAttachment` true :`RelativeTransform` (`KismetMathLibrary.MakeTransform` (0.0 0.0 0.0))))
                  (`SceneComponent.K2_AttachToComponent` _returnvalue_2 (`self.TetherFromComp`) "None" "KeepRelative" "KeepRelative" "KeepRelative" true)
                  (`PhysicsConstraintComponent.SetConstrainedComponents` _returnvalue_2 (`self.TetherFromComp`) "None" (`KismetArrayLibrary.Array_Get` (`self.Joints`)) "None")
                  (`SceneComponent.SetHiddenInGame` _returnvalue_2 false false))
                (:`then_1`
                  (for _index_2 (range (`KismetArrayLibrary.Array_LastIndex` (`self.Joints`)))
                    (bind _returnvalue_3 (`AddComponent|NODE_AddPhysicsConstraintComponent-4` :`bManualAttachment` true :`RelativeTransform` (`KismetMathLibrary.MakeTransform` (0.0 0.0 0.0))))
                    (bind _item_2 (`KismetArrayLibrary.Array_Get` _joints _index_2))
                    (`SceneComponent.K2_AttachToComponent` _returnvalue_3 _item_2 "None" "KeepRelative" "KeepRelative" "KeepRelative" true)
                    (`PhysicsConstraintComponent.SetConstrainedComponents` _returnvalue_3 _item_2 "None" (`KismetArrayLibrary.Array_Get` _joints (+ _index_2 1)) "None")))
                (:`then_2`
                  (bind _asstatic_mesh_component (cast `StaticMeshComponent` (`self.TetherToComp`)))
                  (bind _returnvalue_4 (`AddComponent|NODE_AddPhysicsConstraintComponent-6` :`bManualAttachment` true :`RelativeTransform` (`KismetMathLibrary.MakeTransform` (0.0 0.0 0.0))))
                  (`SceneComponent.K2_AttachToComponent` _returnvalue_4 _item "None" "KeepRelative" "KeepRelative" "KeepRelative" true)
                  (`PhysicsConstraintComponent.SetConstrainedComponents` _returnvalue_4 _item "None" _asstatic_mesh_component "None"))))))))))

(fn `UserConstructionScript`
  (`self.UpdateReferences`))