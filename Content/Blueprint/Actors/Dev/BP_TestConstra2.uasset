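; Dev test actor for tethering with a physics constraint between two helper meshes.
; On BeginPlay it attaches and welds the start mesh to TetherFrom's root and the end mesh to the start mesh, then sets both as the constrained components.
; TetherTo appears only in disconnected experiments, and the construction script and UpdateAttachment are empty apart from similar unused nodes.
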(event `self.ReceiveBeginPlay`
  (`SceneComponent.K2_AttachToComponent` (`self.ConstraAttachMesh`) (`self.K2_GetRootComponent` (`self.TetherFrom`)) "None" "KeepWorld" "KeepWorld" "KeepWorld" true)
  (`SceneComponent.K2_AttachToComponent` (`self.ConstraEndMesh`) (`self.ConstraAttachMesh`) "None" "KeepWorld" "KeepWorld" "KeepWorld" true)
  (`PhysicsConstraintComponent.SetConstrainedComponents` (`self.PhysicsConstraint`) (`self.ConstraAttachMesh`) "None" (`self.ConstraEndMesh`) "None"))

(fn `UpdateAttachment`)

(fn `UserConstructionScript`)