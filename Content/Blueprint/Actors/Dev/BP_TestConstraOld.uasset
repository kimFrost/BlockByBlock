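; Dev test actor that tethers two referenced actors, TetherFrom and TetherTo, with a physics constraint.
; Both the construction script and BeginPlay cast each actor's root to a static mesh component, attach the constraint to the TetherFrom mesh keeping world location, and set the two meshes as constrained components.
; UpdateAttachment is an empty stub with disconnected leftover nodes.
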(event `self.ReceiveBeginPlay`
  (bind _tetherto (`self.TetherTo`))
  (bind _physicsconstraint (`self.PhysicsConstraint`))
  (`/Engine/EditorBlueprintResources/StandardMacros.IsValid` (`self.TetherFrom`)
    (:`Is Valid`
      (`/Engine/EditorBlueprintResources/StandardMacros.IsValid` _tetherto
        (:`Is Valid`
          (bind _asstatic_mesh_component (cast `StaticMeshComponent` (`self.K2_GetRootComponent` (`self.TetherFrom`))))
          (bind _asstatic_mesh_component_2 (cast `StaticMeshComponent` (`self.K2_GetRootComponent` _tetherto)))
          (`SceneComponent.K2_AttachToComponent` _physicsconstraint _asstatic_mesh_component "None" "KeepWorld" "KeepRelative" "KeepRelative" false)
          (`PhysicsConstraintComponent.SetConstrainedComponents` _physicsconstraint _asstatic_mesh_component "None" _asstatic_mesh_component_2 "None"))))))

(fn `UpdateAttachment`)

(fn `UserConstructionScript`
  (bind _physicsconstraint (`self.PhysicsConstraint`))
  (`/Engine/EditorBlueprintResources/StandardMacros.IsValid` (`self.TetherFrom`)
    (:`Is Valid`
      (`/Engine/EditorBlueprintResources/StandardMacros.IsValid` (`self.TetherTo`)
        (:`Is Valid`
          (bind _asstatic_mesh_component (cast `StaticMeshComponent` (`self.K2_GetRootComponent` (`self.TetherFrom`))))
          (bind _asstatic_mesh_component_2 (cast `StaticMeshComponent` (`self.K2_GetRootComponent` (`self.TetherTo`))))
          (`SceneComponent.K2_AttachToComponent` _physicsconstraint _asstatic_mesh_component "None" "KeepWorld" "KeepRelative" "KeepRelative" false)
          (`PhysicsConstraintComponent.SetConstrainedComponents` _physicsconstraint _asstatic_mesh_component "None" _asstatic_mesh_component_2 "None"))))))