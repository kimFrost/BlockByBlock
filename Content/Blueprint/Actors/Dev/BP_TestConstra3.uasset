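; Dev test actor that builds a physics-constraint tether between two actors, TetherFrom and TetherTo.
; Four joint components are spaced evenly along the straight line between them, both in the construction script and again at BeginPlay.
; BeginPlay then links start actor, joints and end actor into a constraint chain, requiring both actors to have static mesh roots.
; UpdateAttachment is an empty stub with unconnected leftover nodes.
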(event `self.ReceiveBeginPlay`
  (`/Engine/EditorBlueprintResources/StandardMacros.IsValid` (`self.TetherFrom`)
    (:`Is Valid`
      (`/Engine/EditorBlueprintResources/StandardMacros.IsValid` (`self.TetherTo`)
        (:`Is Valid`
          (bind _asstatic_mesh_component (cast `StaticMeshComponent` (`self.K2_GetRootComponent` (`self.TetherFrom`))))
          (bind _asstatic_mesh_component_2 (cast `StaticMeshComponent` (`self.K2_GetRootComponent` (`self.TetherTo`))))
          (`self.UpdateJointPlacement`)
          (`PhysicsConstraintComponent.SetConstrainedComponents` (`self.StartConstraint`) _asstatic_mesh_component "None" (`self.Joint1`) "None")
          (`PhysicsConstraintComponent.SetConstrainedComponents` (`self.Joint1Constraint`) (`self.Joint1`) "None" (`self.Joint2`) "None")
          (`PhysicsConstraintComponent.SetConstrainedComponents` (`self.Joint2Constraint`) (`self.Joint2`) "None" (`self.Joint3`) "None")
          (`PhysicsConstraintComponent.SetConstrainedComponents` (`self.Joint3Constraint`) (`self.Joint3`) "None" (`self.Joint4`) "None")
          (`PhysicsConstraintComponent.SetConstrainedComponents` (`self.Joint4Constraint`) (`self.Joint4`) "None" _asstatic_mesh_component_2 "None"))))))

(fn `UpdateAttachment`)

(fn `UpdateJointPlacement`
  (bind _returnvalue (`self.K2_GetActorLocation` (`self.TetherFrom`)))
  (bind _returnvalue_2 (`self.K2_GetActorLocation` (`self.TetherTo`)))
  (set `self.DirectionVector` (`KismetMathLibrary.GetDirectionUnitVector` _returnvalue _returnvalue_2))
  (set `self.Length` (`KismetMathLibrary.VSize` (- _returnvalue _returnvalue_2)))
  (set `self.JointSpacingVector` (* (`self.DirectionVector`) (/ (`self.Length`) 5.0)))
  (`SceneComponent.K2_SetWorldLocation` (`self.Joint1`) (+ (`self.K2_GetActorLocation` (`self.TetherFrom`)) (`self.JointSpacingVector`)) false true)
  (`SceneComponent.K2_SetWorldLocation` (`self.Joint2`) (+ (`self.K2_GetActorLocation` (`self.TetherFrom`)) (* (`self.JointSpacingVector`) 2.0)) false true)
  (`SceneComponent.K2_SetWorldLocation` (`self.Joint3`) (+ (`self.K2_GetActorLocation` (`self.TetherFrom`)) (* (`self.JointSpacingVector`) 3.0)) false true)
  (`SceneComponent.K2_SetWorldLocation` (`self.Joint4`) (+ (`self.K2_GetActorLocation` (`self.TetherFrom`)) (* (`self.JointSpacingVector`) 4.0)) false true))

(fn `UserConstructionScript`
  (`/Engine/EditorBlueprintResources/StandardMacros.IsValid` (`self.TetherFrom`)
    (:`Is Valid`
      (`/Engine/EditorBlueprintResources/StandardMacros.IsValid` (`self.TetherTo`)
        (:`Is Valid`
          (`self.UpdateJointPlacement`))))))