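; BP_Belt is a conveyor actor that shuttles a single BlockSlot child actor between FromLocation and ToLocation to deliver blocks.
; On BeginPlay it derives travel time from distance and Speed, then loops latent MoveComponentTo moves with short delays.
; At the far end the slot tips up, calls ReleaseBlock on its BP_BlockSlot, settles and travels back.
; InterpToMovement, release force and construction-time multi-slot spawning are present but disconnected.
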(event `self.ReceiveBeginPlay`
  (bind _output_get (set `self.Distance` (`KismetMathLibrary.VSize` (- (`self.FromLocation`) (`self.ToLocation`)))))
  (set `self.TravelTime` (/ _output_get (`self.Speed`)))
  (`KismetSystemLibrary.MoveComponentTo` (`self.BlockSlot`) (- (`self.ToLocation`) (`self.K2_GetActorLocation`)) (struct) false false (`self.TravelTime`) :!label _label)
  (`KismetSystemLibrary.Delay` 0.2)
  (`KismetSystemLibrary.MoveComponentTo` (`self.BlockSlot`) (+ (- (`self.ToLocation`) (`self.K2_GetActorLocation`)) (0.0 0.0 50.0)) (struct :`Roll` 50.0) false false 0.1)
  (bind _asbp_block_slot (cast `/Game/Blueprint/Actors/BP_BlockSlot` (`ChildActorComponent.ChildActor` (`self.BlockSlot`))))
  (bind (_breleased _releasedblock) (`/Game/Blueprint/Actors/BP_BlockSlot.ReleaseBlock` _asbp_block_slot true))
  (`KismetSystemLibrary.Delay` 0.2)
  (`KismetSystemLibrary.MoveComponentTo` (`self.BlockSlot`) (- (`self.ToLocation`) (`self.K2_GetActorLocation`)) (struct) false false 0.5)
  (`KismetSystemLibrary.Delay` 0.5)
  (`KismetSystemLibrary.MoveComponentTo` (`self.BlockSlot`) (- (`self.FromLocation`) (`self.K2_GetActorLocation`)) (struct) false false (`self.TravelTime`))
  (`KismetSystemLibrary.Delay` 1.0)
  (goto _label))

(fn `UserConstructionScript`)