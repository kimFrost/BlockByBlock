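; BP_BlockSlot is an actor that holds one BP_Block at an attach point, optionally catching eligible blocks that overlap its box.
; AddBlock fastens and attaches a block, then a timeline eases it into place.
; ReleaseBlock detaches it, optionally loosens it, and starts a cooldown that pauses overlap pickup.
; Both fire dispatchers, and queries first clear any block reference no longer attached to the slot.
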(event `self.ReceiveBeginPlay`
  (if (not (`self.BlotSlotHasCollision`))
    (`PrimitiveComponent.SetCollisionResponseToChannel` (`self.BlockSlot`) "ECC_Pawn" "ECR_Ignore")))

(event `self.Box.OnComponentBeginOverlap`
  (params (OverlappedComponent :type "PrimitiveComponent Object Reference") (OtherActor :type "Actor Object Reference") (OtherComp :type "PrimitiveComponent Object Reference") (OtherBodyIndex :type Integer) (bFromSweep :type Boolean) (SweepResult :type "HitResult Structure (by ref)"))
  (if (`self.TraceForBlocks`)
    (if (not (`self.AddCooldowmInEffect`))
      (bind _asbp_block (cast `/Game/Blueprint/Actors/BP_Block` OtherActor))
      (if (`/Game/Blueprint/Actors/BP_Block.CanBeTracePickedUp` _asbp_block)
        (`self.AddBlock` _asbp_block)))))

(event `MoveBlockToSlot`
  (params (Block :type "/Game/Blueprint/Actors/BP_Block Object Reference"))
  (bind _block (`self.Block`))
  (bind _block_2 (`self.Block`))
  (bind _block_3 (`self.Block`))
  (`/Engine/EditorBlueprintResources/StandardMacros.IsValid` Block
    (:`Is Valid`
      (`/Game/Blueprint/Actors/BP_Block.DisableCollision` Block)
      (bind (_direction _alpha) (`Timeline|Timeline_0` :`NewTime` 1.0 :!via `PlayFromStart`)
        (:`Update`
          (`/Engine/EditorBlueprintResources/StandardMacros.IsValid` (`self.Block`)
            (:`Is Valid`
              (`self.K2_SetActorLocation` _block_3 (`KismetMathLibrary.VLerp` (`self.K2_GetActorLocation` _block_2) (`SceneComponent.K2_GetComponentLocation` (`self.AttachPoint`)) _alpha) false false)
              (`self.K2_SetActorRotation` _block_3 (`KismetMathLibrary.RLerp` (`self.K2_GetActorRotation` _block_2) (`SceneComponent.K2_GetComponentRotation` (`self.AttachPoint`)) _alpha true) false))))
        (:`Finished`
          (`/Engine/EditorBlueprintResources/StandardMacros.IsValid` _block
            (:`Is Valid`
              (if (`self.BlockHasCollision`)
                (`/Game/Blueprint/Actors/BP_Block.EnableCollision` _block)
                (else
                  (`/Game/Blueprint/Actors/BP_Block.DisableCollision` _block))))))))))

(event `StartAddCooldown`
  (set `self.AddCooldowmInEffect` true)
  (`Timeline|Timeline_AddCooldown` :`NewTime` 1.0 :!via `PlayFromStart`
    (:`Finished`
      (set `self.AddCooldowmInEffect` false))))

(fn `AddBlock`
  (params (Block :type "/Game/Blueprint/Actors/BP_Block Object Reference"))
  (returns (bAdded :type Boolean))
  (bind _block (`self.Block`))
  (`self.ValidateAttached`)
  (`/Engine/EditorBlueprintResources/StandardMacros.IsValid` (`self.Block`)
    (:`Is Valid`
      _)
    (:`Is Not Valid`
      (`/Engine/EditorBlueprintResources/StandardMacros.IsValid` Block
        (:`Is Valid`
          (`self.K2_AttachToComponent` Block (`self.AttachPoint`) "None" "KeepWorld" "KeepWorld" "KeepWorld" true)
          (set `self.Block` Block)
          (`/Game/Blueprint/Actors/BP_Block.FastenBlock` (`self.Block`))
          (if (`self.BlockHasCollision`)
            (`/Game/Blueprint/Actors/BP_Block.EnableCollision` _block)
            (else
              (`/Game/Blueprint/Actors/BP_Block.DisableCollision` _block)))
          (`self.OnBlockAdded` (`self.Block`))
          (`self.MoveBlockToSlot` (`self.Block`))
          (return true))
        (:`Is Not Valid`
          _))))
  (return false))

(fn `IsFree`
  (returns (IsFree :type Boolean))
  (`self.ValidateAttached`)
  (`/Engine/EditorBlueprintResources/StandardMacros.IsValid` (`self.Block`)
    (:`Is Valid`
      (return false))
    (:`Is Not Valid`
      (return true))))

(fn `ReleaseBlock`
  (params (bLoosen :type Boolean))
  (returns (bReleased :type Boolean) (ReleasedBlock :type "/Game/Blueprint/Actors/BP_Block Object Reference"))
  (locals (Local_ReleasedBlock :type "/Game/Blueprint/Actors/BP_Block Object Reference"))
  (bind _block (`self.Block`))
  (bind _local_releasedblock (`local.Local_ReleasedBlock`))
  (`self.ValidateAttached`)
  (`/Engine/EditorBlueprintResources/StandardMacros.IsValid` _block
    (:`Is Valid`
      (`self.K2_DetachFromActor` _block "KeepWorld" "KeepWorld" "KeepWorld")
      (set `local.Local_ReleasedBlock` (`self.Block`))
      (set `self.Block` null)
      (`self.StartAddCooldown`)
      (if bLoosen
        (`/Game/Blueprint/Actors/BP_Block.LoosenBlock` _local_releasedblock))
      (`self.OnBlockReleased` _local_releasedblock)
      (return true _local_releasedblock))
    (:`Is Not Valid`
      (return false null))))

(fn `UserConstructionScript`)

(fn `ValidateAttached`
  (bind _block (`self.Block`))
  (`/Engine/EditorBlueprintResources/StandardMacros.IsValid` _block
    (:`Is Valid`
      (if (not (== (`self.AttachPoint`) (`SceneComponent.GetAttachParent` (`/Game/Blueprint/Actors/BP_Block.StaticMesh` _block))))
        (set `self.Block` null)))))