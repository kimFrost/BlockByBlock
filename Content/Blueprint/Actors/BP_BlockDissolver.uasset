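; BP_BlockDissolver is an actor that consumes blocks placed into its slot and awards the player a point for each.
; On BeginPlay it binds to the OnBlockAdded event of the BP_BlockSlot held in its child actor component.
; When a valid block arrives, it waits briefly, adds a point through BlockByBlockGameMode, then destroys the block.
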(event `self.ReceiveBeginPlay`
  (bind _asbp_block_slot (cast `/Game/Blueprint/Actors/BP_BlockSlot` (`ChildActorComponent.ChildActor` (`self.ChildActor`))))
  (add `/Game/Blueprint/Actors/BP_BlockSlot.OnBlockAdded` _asbp_block_slot (delegate `CustomEvent_0`)))

(event `CustomEvent_0`
  (params (Block :type "/Game/Blueprint/Actors/BP_Block Object Reference"))
  (`/Engine/EditorBlueprintResources/StandardMacros.IsValid` Block
    (:`Is Valid`
      (`KismetSystemLibrary.Delay` 0.5)
      (bind _asblock_by_block_game_mode (cast `BlockByBlockGameMode` (`GameplayStatics.GetGameMode`)))
      (`BlockByBlockGameMode.AddPoints` _asblock_by_block_game_mode 1)
      (`self.K2_DestroyActor` Block))))

(fn `UserConstructionScript`)