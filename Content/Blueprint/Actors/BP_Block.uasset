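; Block actor that can be knocked loose into physics simulation, with optional interpolated movement.
; Construction sets the initial physics state, and BeginPlay starts InterpToMovement when Move is set.
; AddForceToBlock acts only on non-simulating blocks: LoosenBlock shrinks the mesh slightly and enables physics, then force is applied as an acceleration change.
; UpdateAdjacentBlocks is an empty stub, and several events only print debug text, including Tick every frame.
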(event `self.ReceiveBeginPlay`
  (if (`self.Move`)
    (`ActorComponent.Activate` (`self.InterpToMovement`) true)))

(event `self.ReceiveTick`
  (params (DeltaSeconds :type "Float (single-precision)"))
  (`KismetSystemLibrary.PrintString` "Hello" true true (struct :`G` 0.66 :`B` 1.0 :`A` 1.0) 0.0))

(event `self.StaticMesh.PhysicsVolumeChangedDelegate`
  (params (NewVolume :type "PhysicsVolume Object Reference"))
  (`KismetSystemLibrary.PrintString` "add force 1"))

(event `self.StaticMesh.OnComponentHit`
  (params (HitComponent :type "PrimitiveComponent Object Reference") (OtherActor :type "Actor Object Reference") (OtherComp :type "PrimitiveComponent Object Reference") (NormalImpulse :type "Vector Structure") (Hit :type "HitResult Structure (by ref)")))

(event `self.StaticMesh.OnComponentWake`
  (params (WakingComponent :type "PrimitiveComponent Object Reference") (BoneName :type Name))
  (`KismetSystemLibrary.PrintString` "block wake"))

(fn `AddForceToBlock`
  (params (Force :type "Vector Structure"))
  (if (not (`SceneComponent.IsSimulatingPhysics` (`self.StaticMesh`) "None"))
    (`self.LoosenBlock`)
    (`PrimitiveComponent.AddForce` (`self.StaticMesh`) Force "None" true)))

(fn `LoosenBlock`
  (bind _staticmesh (`self.StaticMesh`))
  (`SceneComponent.SetWorldScale3D` _staticmesh (0.98 0.98 0.98))
  (`PrimitiveComponent.SetSimulatePhysics` _staticmesh true)
  (`self.UpdateAdjacentBlocks`))

(fn `UpdateAdjacentBlocks`)

(fn `UserConstructionScript`
  (`PrimitiveComponent.SetSimulatePhysics` (`self.StaticMesh`) (`self.SimulatePhysics`)))