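; BP_Cart is a cart actor that places itself on a rail path when play begins.
; A complex downward line trace with persistent debug drawing looks for a BP_RailPath beneath it, then teleports the cart slightly above that actor's origin, not the hit point.
; Each tick clamps the cart's pitch while keeping roll and yaw, applying the rotation as a physics teleport.
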(event `self.ReceiveBeginPlay`
  (`self.TraceForTracks`))

(event `self.ReceiveTick`
  (params (DeltaSeconds :type "Float (single-precision)"))
  (`self.K2_SetActorRotation` (`KismetMathLibrary.MakeRotator` (.roll (`self.K2_GetActorRotation`)) (`KismetMathLibrary.FClamp` (.pitch (`self.K2_GetActorRotation`)) -50.0 50.0) (.yaw (`self.K2_GetActorRotation`))) true))

(fn `TraceForTracks`
  (bind _returnvalue (`self.K2_GetActorLocation`))
  (bind (_outhit _returnvalue_2) (`KismetSystemLibrary.LineTraceSingle` :`Start` _returnvalue :`End` (+ _returnvalue (0.0 0.0 -1000.0)) :`TraceChannel` "TraceTypeQuery1" :`bTraceComplex` true :`DrawDebugType` "Persistent"))
  (if _returnvalue_2
    (bind (_bblockinghit _binitialoverlap _time _location _impactpoint _normal _impactnormal _physmat _hitactor) (`GameplayStatics.BreakHitResult` _outhit))
    (cast `/Game/Blueprint/Actors/Dev/BP_RailPath` _hitactor)
    (`self.K2_SetActorLocation` (+ (`self.K2_GetActorLocation` _hitactor) (0.0 0.0 50.0)) false true)))

(fn `UserConstructionScript`)